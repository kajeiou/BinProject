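; MyBP_Spot is a light spot actor with a sphere mesh and a point light, either fixed or interactive depending on the SpotInteractif flag.
; On BeginPlay, a fixed spot starts lit with the spot material, while an interactive one starts dark with a gray material.
; SphereCollision overlap events light an interactive spot when the first-person character enters and switch it off when the character leaves.
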(event `self.ReceiveBeginPlay`
  (bind _sphere (`self.Sphere`))
  (bind _pointlight (`self.PointLight`))
  (if (`self.SpotInteractif`)
    ;[1 1 1] Initialisation d'un point lumineux interactif
    (`PrimitiveComponent.SetMaterial` _sphere 0 "/Game/LevelPrototyping/Materials/MI_PrototypeGrid_Gray.MI_PrototypeGrid_Gray")
    (`LightComponent.SetIntensity` _pointlight 0.0)
    (else
      ;[1 1 1] Initialisation d'un point lumineux fixe
      (`PrimitiveComponent.SetMaterial` _sphere 0 "/Game/MyAssets/Materials/MyMat_Spot.MyMat_Spot")
      (`LightComponent.SetIntensity` _pointlight 5000.0))))

(event `self.SphereCollision.OnComponentBeginOverlap`
  (params (OverlappedComponent :type "PrimitiveComponent Object Reference") (OtherActor :type "Actor Object Reference") (OtherComp :type "PrimitiveComponent Object Reference") (OtherBodyIndex :type Integer) (bFromSweep :type Boolean) (SweepResult :type "HitResult Structure (by ref)"))
  ;[1 1 1] Allumage d'un point lumineux interactif
  (cast `/Game/FirstPerson/Blueprints/BP_FirstPersonCharacter` OtherActor)
  (if (`self.SpotInteractif`)
    (`LightComponent.SetIntensity` (`self.PointLight`) 5000.0)
    (`PrimitiveComponent.SetMaterial` (`self.Sphere`) 0 "/Game/MyAssets/Materials/MyMat_Spot.MyMat_Spot")))

(event `self.SphereCollision.OnComponentEndOverlap`
  (params (OverlappedComponent :type "PrimitiveComponent Object Reference") (OtherActor :type "Actor Object Reference") (OtherComp :type "PrimitiveComponent Object Reference") (OtherBodyIndex :type Integer))
  ;[1 1 1] Extinction d'un point lumineux interactif
  (cast `/Game/FirstPerson/Blueprints/BP_FirstPersonCharacter` OtherActor)
  (if (`self.SpotInteractif`)
    (`LightComponent.SetIntensity` (`self.PointLight`) 0.0)
    (`PrimitiveComponent.SetMaterial` (`self.Sphere`) 0 "/Game/LevelPrototyping/Materials/MI_PrototypeGrid_Gray.MI_PrototypeGrid_Gray")))

(fn `UserConstructionScript`)